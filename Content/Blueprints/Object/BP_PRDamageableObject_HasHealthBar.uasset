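; BP_PRDamageableObject_HasHealthBar is a damageable world object that shows damage numbers and is destroyed when its health runs out.
; TakeDamage spawns a BP_PRDamageAmount actor, initialized with the hit's impact location, amount, critical flag and element.
; It then subtracts the amount from current health, destroys the actor at zero or below, and returns true.
; Event graph and construction script are empty, and no health bar logic appears here despite the name.
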(fn `TakeDamage`
  (params (DamageInfo :type "PRDamageInfo Structure"))
  (returns (ReturnValue :type Boolean))
  (bind (_amount _damagetype _damageelement _damageresponse _impactlocation _biscritical) (break `PRDamageInfo` DamageInfo))
  (bind _returnvalue (`|SpawnActorFromClass` "/Game/Blueprints/Object/BP_PRDamageAmount.BP_PRDamageAmount_C" (`self.GetTransform`) "Undefined" "MultiplyWithRoot" null null))
  (`PRDamageAmount.Initialize` _returnvalue _impactlocation _amount _biscritical _damageelement)
  (bind _returnvalue_2 (`Interface_PRDamageable.GetCurrentHealth`))
  (bind _output_get (set `self.Health` (- _returnvalue_2 _amount)))
  (if (<= _output_get 0.0)
    (`self.K2_DestroyActor`))
  (return true))

(fn `UserConstructionScript`)