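; BP_PRPlayerCharacter_SingleSword is the single-sword player character Blueprint, whose graph holds only debug hooks for the EffectSystem's pooled Niagara effects.
; Numpad 7, 8 and 9 spawn shockwave, weapon-spawn and placeholder Niagara effects through EffectSystem.
; Tick loops over the NiagaraEffectPool keys and prints a default message for each valid one.
; A detailed print of each effect's activation state and pool index is left disconnected.
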(event `self.ReceiveBeginPlay`)

(event `self.ReceiveTick`
  (params (DeltaSeconds :type "Float (single-precision)"))
  (bind _keys (`BlueprintMapLibrary.Map_Keys` (`PREffectSystemComponent.NiagaraEffectPool` (`self.EffectSystem`))))
  (for _array_element _keys
    (`/Engine/EditorBlueprintResources/StandardMacros.IsValid` _array_element
      (:`Is Valid`
        (`KismetSystemLibrary.PrintString` "Hello" true true (struct :`G` 0.66 :`B` 1.0 :`A` 1.0) 0.0)))))

(event `Key|NumPadSeven`
  (params (Key :type "Key Structure"))
  (:`Pressed`
    (`PREffectSystemComponent.SpawnNiagaraEffectAtLocation` :`self` (`self.EffectSystem`) :`SpawnEffect` "/Game/VFX/Player/DoubleJump/New/NS_DoubleJumpShockwave.NS_DoubleJumpShockwave")))

(event `Key|NumPadNine`
  (params (Key :type "Key Structure"))
  (:`Pressed`
    (`PREffectSystemComponent.SpawnNiagaraEffectAtLocation` :`self` (`self.EffectSystem`) :`SpawnEffect` "/Game/VFX/Player/DoubleJump/NewNiagaraSystem.NewNiagaraSystem")))

(event `Key|NumPadEight`
  (params (Key :type "Key Structure"))
  (:`Pressed`
    (`PREffectSystemComponent.SpawnNiagaraEffectAtLocation` :`self` (`self.EffectSystem`) :`SpawnEffect` "/Game/VFX/SpawnWeapon/NS_SpawnWeapon.NS_SpawnWeapon")))

(fn `UserConstructionScript`)